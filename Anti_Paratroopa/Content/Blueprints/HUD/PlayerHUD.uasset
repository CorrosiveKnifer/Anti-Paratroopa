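; Player HUD for a flying combat game that creates the crosshair, bounds and pause widgets and toggles them with the game mode's pause state.
; A looping timer finds the nearest Enemy, and Tick projects it to screen to place the clamped crosshair, flagging it on target when centred and in range.
; Tick also stores the aim location, defaulting to camera-forward without a target, and hides crosshair and bounds when no Plane exists.
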(event EventBeginPlay
  (bind _returnvalue (Game|GetPlayerController 0))
  (bind _returnvalue_2 (Game|GetPlayerController 0))
  (Utilities|IsValid _returnvalue
    (:Is%20Valid
      (Input|SetInputModeGameOnly _returnvalue)
      (Utilities|Time|SetTimerbyFunctionName 0 "FindNearestEnemy" 0.05 true)
      (bind _returnvalue_3 (UserInterface|CreateWidget "/Game/Blueprints/Widgets/MainGame/PlayerCross.PlayerCross_C" _returnvalue_2))
      (bind _output_get (Variables|Default|SetCrossHair _returnvalue_3))
      (UserInterface|Viewport|AddtoViewport _output_get 0)
      (bind _returnvalue_4 (UserInterface|CreateWidget "/Game/Blueprints/Widgets/MainGame/PlayerBounds.PlayerBounds_C" _returnvalue_2))
      (bind _output_get_2 (Variables|Default|SetUI _returnvalue_4))
      (UserInterface|Viewport|AddtoViewport _output_get_2 0)
      (bind _returnvalue_5 (UserInterface|CreateWidget "/Game/Blueprints/Widgets/MainGame/Pause.Pause_C" _returnvalue_2))
      (bind _output_get_3 (Variables|Default|SetPause _returnvalue_5))
      (UserInterface|Viewport|AddtoViewport _output_get_3 0)
      (Widget|SetVisibility _output_get_3 "Hidden"))))

(event EventTick
  (params (DeltaSeconds :type Float%20%28single-precision%29))
  (bind _returnvalue (Game|GetPlayerCameraManager 0))
  (bind _returnvalue_2 (Viewport|GetViewportSize))
  (bind _returnvalue_3 (Class|WidgetLayoutLibrary|GetViewportScale))
  (bind _returnvalue_4 (Game|GetPlayerController 0))
  (bind _nearestenemy (Variables|Default|GetNearestEnemy))
  (bind _returnvalue_5 (- (.y _returnvalue_2) 22.5))
  (bind _returnvalue_6 (- (.x _returnvalue_2) 22.5))
  (bind _returnvalue_7 (Transformation|GetActorLocation _nearestenemy))
  (bind _returnvalue_8 (* _returnvalue_3 22.5))
  (bind _screenlocation (Class|PlayerController|ProjectWorldLocationtoScreen _returnvalue_4 _returnvalue_7 false))
  (bind _returnvalue_9 (- (.y _screenlocation) _returnvalue_8))
  (bind _returnvalue_10 (- (.x _screenlocation) _returnvalue_8))
  (bind _returnvalue_11 (Math|Float|Clamp(Float) _returnvalue_9 0.0 _returnvalue_5))
  (bind _returnvalue_12 (Math|Float|Clamp(Float) _returnvalue_10 0.0 _returnvalue_6))
  (bind _outactors (Actor|GetAllActorsOfClass "/Game/Blueprints/Plane.Plane_C"))
  (if (> (Utilities|Array|Length _outactors) 0)
    (bind _asflying_game_mode (Utilities|Casting|CastToFlyingGameMode (Game|GetGameMode)))
    (CallFunction|PauseVis (Variables|/Game/Blueprints/Gamemodes/FlyingGameMode.FlyingGameMode_C|GetUserPaused _asflying_game_mode))
    (else
      (Widget|SetVisibility (Variables|Default|GetCrossHair) "Hidden")))
  (Utilities|IsValid (Variables|Default|GetNearestEnemy)
    (:Is%20Valid
      (CallFunction|IsCrossRed _returnvalue_12 _returnvalue_11 (Variables|Default|GetEnemyDistance))
      (bind _asflying_game_mode_2 (Utilities|Casting|CastToFlyingGameMode (Game|GetGameMode)))
      (Variables|/Game/Blueprints/Gamemodes/FlyingGameMode.FlyingGameMode_C|SetClosestEnemyDistance _asflying_game_mode_2 (Variables|Default|GetEnemyDistance))
      (Class|UserWidget|SetPositioninViewport (Variables|Default|GetCrossHair) (Math|Vector2D|MakeVector2D _returnvalue_12 _returnvalue_11) true)
      (Variables|Default|SetCrossLoc _returnvalue_7))
    (:Is%20Not%20Valid
      (bind _asplayer_cross (Utilities|Casting|CastToPlayerCross (Variables|Default|GetCrossHair)))
      (Variables|/Game/Blueprints/Widgets/MainGame/PlayerCross.PlayerCross_C|SetIsOnTarget _asplayer_cross true)
      (bind _asflying_game_mode_3 (Utilities|Casting|CastToFlyingGameMode (Game|GetGameMode)))
      (Variables|/Game/Blueprints/Gamemodes/FlyingGameMode.FlyingGameMode_C|SetClosestEnemyDistance _asflying_game_mode_3 0.0)
      (Class|UserWidget|SetPositioninViewport (Variables|Default|GetCrossHair) (- (/ (Math|Vector2D|MakeVector2D (.x _returnvalue_2) (.y _returnvalue_2)) 2.0) "(X=22.500000,Y=22.500000)") true)
      (Variables|Default|SetCrossLoc (+ (Transformation|GetActorLocation _returnvalue) (* (Math|Vector|GetForwardVector (Variables|/Script/Engine.Actor|GetRootComponent _returnvalue)) 1.5e+04))))))

(fn ConstructionScript)

(fn FindNearestEnemy
  (Utilities|IsValid (Game|Player|GetPlayerPawn 0)
    (:Is%20Valid
      (bind _outactors (Actor|GetAllActorsOfClass "/Game/Blueprints/Enemy.Enemy_C"))
      (if (> (Utilities|Array|Length _outactors) 0)
        ;[1 1 1] Set first index as "base" to compare to
        (Variables|Default|SetNearestEnemy (Utilities|Array|Get(acopy) _outactors))
        (Variables|Default|SetEnemyDistance (Transformation|GetDistanceTo (Game|Player|GetPlayerPawn 0) (Utilities|Array|Get(acopy) _outactors)))
        (for (_ _array_index) _outactors
          (if (< (Transformation|GetDistanceTo (Game|Player|GetPlayerPawn 0) (Utilities|Array|Get(acopy) _outactors _array_index)) (Variables|Default|GetEnemyDistance))
            (Variables|Default|SetNearestEnemy (Utilities|Array|Get(acopy) _outactors _array_index))
            (Variables|Default|SetEnemyDistance (Transformation|GetDistanceTo (Game|Player|GetPlayerPawn 0) (Utilities|Array|Get(acopy) _outactors _array_index)))))))))

(fn IsCrossRed
  (params (x :type Float%20%28single-precision%29) (y :type Float%20%28single-precision%29) (distance :type Float%20%28single-precision%29))
  (bind _returnvalue (Viewport|GetViewportSize))
  (bind _bounds (LocalVariables|GetBounds))
  (bind _returnvalue_2 (/ _returnvalue 2.0))
  (bind (_x _y) (Math|Vector2D|BreakVector2D _returnvalue_2))
  (bind _asplayer_cross (Utilities|Casting|CastToPlayerCross (Variables|Default|GetCrossHair))
    (:then
      (bind _output_get (Variables|/Game/Blueprints/Widgets/MainGame/PlayerCross.PlayerCross_C|SetIsOnTarget _asplayer_cross (Math|Boolean|ANDBoolean (<= x (+ _x _bounds)) (>= x (- _x _bounds)) (<= y (+ _y _bounds)) (>= y (- _y _bounds)) (<= distance 2.5e+04))))
      (return _output_get))
    (:CastFailed
      (return false))))

(fn PauseVis
  (params (IsVisible :type Boolean))
  (bind _crosshair (Variables|Default|GetCrossHair))
  (bind _ui (Variables|Default|GetUI))
  (bind _pause (Variables|Default|GetPause))
  (if IsVisible
    (Widget|SetVisibility _pause "Visible")
    (Widget|SetVisibility _ui "Hidden")
    (Widget|SetVisibility _crosshair "Hidden")
    (else
      (Widget|SetVisibility _pause "Hidden")
      (Widget|SetVisibility _ui "Visible")
      (Widget|SetVisibility _crosshair "Visible"))))