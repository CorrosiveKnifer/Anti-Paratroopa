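; Menu HUD actor that shows the main menu and instructions screens for the menu game mode.
; On BeginPlay it creates both widgets, hides Instructions, sets UI-only input with a locked mouse and shows the cursor.
; Each Tick it polls the MenuGameMode's CurrentState and toggles which widget is visible, showing the main menu by default.
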(event EventBeginPlay
  (bind _returnvalue (Game|GetPlayerController 0))
  (bind _returnvalue_2 (UserInterface|CreateWidget "/Game/Blueprints/Widgets/Menu/MainMenu.MainMenu_C"))
  (bind _output_get (Variables|Default|SetMain _returnvalue_2))
  (UserInterface|Viewport|AddtoViewport _output_get 0)
  (bind _returnvalue_3 (UserInterface|CreateWidget "/Game/Blueprints/Widgets/Menu/Instructions.Instructions_C"))
  (bind _output_get_2 (Variables|Default|SetInstructions _returnvalue_3))
  (UserInterface|Viewport|AddtoViewport _output_get_2 0)
  (Widget|SetVisibility _output_get_2 "Hidden")
  (Input|SetInputModeUIOnly _returnvalue 0 "LockAlways")
  (Variables|/Script/Engine.PlayerController|SetbShowMouseCursor _returnvalue true))

(event Collision|EventActorBeginOverlap
  (params (OtherActor :type Actor%20Object%20Reference)))

(event EventTick
  (params (DeltaSeconds :type Float%20%28single-precision%29))
  (bind _main (Variables|Default|GetMain))
  (bind _instructions (Variables|Default|GetInstructions))
  (bind _asmenu_game_mode (Utilities|Casting|CastToMenuGameMode (Game|GetGameMode)))
  (switch int (Variables|/Game/Blueprints/Gamemodes/MenuGameMode.MenuGameMode_C|GetCurrentState _asmenu_game_mode)
    (:Default
      (Widget|SetVisibility _main "Visible" :!label _label)
      (Widget|SetVisibility _instructions "Hidden"))
    (:0
      (goto _label))
    (:1
      (Widget|SetVisibility _main "Hidden")
      (Widget|SetVisibility _instructions "Visible"))))

(fn ConstructionScript)