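; Enemy actor for a flying game that reports to FlyingGameMode whether it was killed or landed.
; Each Tick applies a constant upward force to its physics Box and checks its height.
; Dropping to a low Z threshold increments the game mode's Landed count and destroys it.
; GetDamaged subtracts incoming damage from Health, incrementing Kills and destroying the actor when Health is depleted.
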(event EventTick
  (params (DeltaSeconds :type Float%20%28single-precision%29))
  (Physics|AddForce (Variables|Default|GetBox) "0, 0,2000.000000" "None" false)
  (if (<= (.Z (Math|Vector|BreakVector (Transformation|GetActorLocation))) -5e+01)
    (bind _asflying_game_mode (Utilities|Casting|CastToFlyingGameMode (Game|GetGameMode)))
    (Variables|/Game/Blueprints/Gamemodes/FlyingGameMode.FlyingGameMode_C|SetLanded _asflying_game_mode (+ (Variables|/Game/Blueprints/Gamemodes/FlyingGameMode.FlyingGameMode_C|GetLanded _asflying_game_mode) 1))
    (Actor|DestroyActor)))

(fn ConstructionScript)

(fn GetDamaged
  (params (Incoming :type Float%20%28single-precision%29))
  (bind _output_get (Variables|Default|SetHealth (- (Variables|Default|GetHealth) Incoming)))
  (if (<= _output_get 0.0)
    (bind _asflying_game_mode (Utilities|Casting|CastToFlyingGameMode (Game|GetGameMode)))
    (Variables|/Game/Blueprints/Gamemodes/FlyingGameMode.FlyingGameMode_C|SetKills _asflying_game_mode (+ (Variables|/Game/Blueprints/Gamemodes/FlyingGameMode.FlyingGameMode_C|GetKills _asflying_game_mode) 1))
    (Actor|DestroyActor)))