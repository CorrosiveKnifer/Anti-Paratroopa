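; Game mode for a flying game that spawns enemies and rings, tracks win and loss conditions, and handles pausing.
; Looping timers call a shared spawner that picks random, bounds-clamped points around the first Plane's driver at fixed altitude, using an overlap check and collision-safe spawning.
; Tick flags a win from kills, clamps ammo, and destroys the player pawn at the landed limit.
; Pause functions toggle game pause, input mode and cursor.
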(event EventBeginPlay
  (Utilities|Time|SetTimerbyFunctionName 0 "SpawnEnemy" 5.0 true)
  (Utilities|Time|SetTimerbyFunctionName 0 "SpawnRing" 8.0 true))

(event EventTick
  (params (DeltaSeconds :type Float%20%28single-precision%29))
  (bind _returnvalue (Game|Player|GetPlayerPawn 0))
  (Variables|Default|SetGameWin (>= (Variables|Default|GetKills) (Variables|Default|GetWin%20Amount)))
  (Variables|Default|SetPlayerAmmo (Math|Integer|Clamp(Integer) (Variables|Default|GetPlayerAmmo) 0 100))
  (if (>= (Variables|Default|GetLanded) (Variables|Default|GetLandedLimit))
    (Utilities|IsValid _returnvalue
      (:Is%20Valid
        (Actor|DestroyActor _returnvalue)))))

(fn ConstructionScript)

(fn SpawnActor
  (params (ToSpawn :type Actor%20Class%20Reference) (Scale :type Vector))
  (bind _x_bounds (Variables|Default|Getx%20bounds))
  (bind _y_bounds (Variables|Default|Gety%20bounds))
  (bind _outactors (Actor|GetAllActorsOfClass "/Game/Blueprints/Plane.Plane_C"))
  (if (> (Utilities|Array|Length _outactors) 0)
    (bind _returnvalue (Collision|SphereOverlapActors (Math|Vector|MakeVector (Math|Float|Clamp(Float) (+ (.x (Transformation|GetWorldLocation (Variables|/Game/Blueprints/Plane.Plane_C|GetDriver (Utilities|Array|Get(acopy) _outactors)))) (Math|Random|RandomFloatinRange -2e+04 2e+04)) (.value (.lowerbound _x_bounds)) (.value (.upperbound _x_bounds))) (Math|Float|Clamp(Float) (+ (.y (Transformation|GetWorldLocation (Variables|/Game/Blueprints/Plane.Plane_C|GetDriver (Utilities|Array|Get(acopy) _outactors)))) (Math|Random|RandomFloatinRange -2e+04 2e+04)) (.value (.lowerbound _y_bounds)) (.value (.upperbound _y_bounds))) 6e+04) 5e+02 (Utilities|Array|MakeArray "ObjectTypeQuery2") 0))
    (if (not _returnvalue)
      (Game|SpawnActorfromClass ToSpawn (Math|Transform|MakeTransform (Math|Vector|MakeVector (Math|Float|Clamp(Float) (+ (.x (Transformation|GetWorldLocation (Variables|/Game/Blueprints/Plane.Plane_C|GetDriver (Utilities|Array|Get(acopy) _outactors)))) (Math|Random|RandomFloatinRange -2e+04 2e+04)) (.value (.lowerbound _x_bounds)) (.value (.upperbound _x_bounds))) (Math|Float|Clamp(Float) (+ (.y (Transformation|GetWorldLocation (Variables|/Game/Blueprints/Plane.Plane_C|GetDriver (Utilities|Array|Get(acopy) _outactors)))) (Math|Random|RandomFloatinRange -2e+04 2e+04)) (.value (.lowerbound _y_bounds)) (.value (.upperbound _y_bounds))) 6e+04) "0, 0, 0" Scale) "DontSpawnIfColliding" 0 0))))

(fn SpawnEnemy
  (CallFunction|SpawnActor "/Game/Blueprints/Enemy.Enemy_C" "0.800000,0.800000,0.800000"))

(fn SpawnRing
  (CallFunction|SpawnActor "/Game/Blueprints/Ring.Ring_C" "15.000000,15.000000,15.000000"))

(fn Pause
  (bind _returnvalue (Game|GetPlayerController 0))
  (Game|SetGamePaused true)
  (Input|SetInputModeUIOnly _returnvalue 0 "LockAlways")
  (Variables|/Script/Engine.PlayerController|SetbShowMouseCursor _returnvalue true)
  (Variables|Default|SetUserPaused true))

(fn UnPause
  (bind _returnvalue (Game|GetPlayerController 0))
  (Game|SetGamePaused false)
  (Input|SetInputModeGameOnly _returnvalue)
  (Variables|/Script/Engine.PlayerController|SetbShowMouseCursor _returnvalue false)
  (Variables|Default|SetUserPaused false))